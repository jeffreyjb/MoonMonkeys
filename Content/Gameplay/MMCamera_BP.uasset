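; MMCamera_BP is a camera actor that makes itself the first player controller's view target on BeginPlay.
; Four directional move functions each offset the root component's relative location when their ShouldMove flag is true.
; Left and Right both add Distance on X, and Up and Down both add it on Y, so direction depends on the sign passed in.
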(event `self.ReceiveBeginPlay`
  (`PlayerController.SetViewTargetWithBlend` (`GameplayStatics.GetPlayerController` 0) self 0.0 "VTBlend_Linear" 0.0 false))

(fn `Move Down`
  (params (Distance :type "Float (double-precision)" :default -10.0) (ShouldMove :type Boolean :default true))
  (if ShouldMove
    (`SceneComponent.K2_AddRelativeLocation` (`self.DefaultSceneRoot`) (`KismetMathLibrary.MakeVector` 0.0 Distance) false false)))

(fn `Move Left`
  (params (Distance :type "Float (double-precision)" :default 10.0) (ShouldMove :type Boolean :default true))
  (if ShouldMove
    (`SceneComponent.K2_AddRelativeLocation` (`self.DefaultSceneRoot`) (`KismetMathLibrary.MakeVector` Distance) false false)))

(fn `Move RIght`
  (params (Distance :type "Float (double-precision)" :default -10.0) (ShouldMove :type Boolean :default true))
  (if ShouldMove
    (`SceneComponent.K2_AddRelativeLocation` (`self.DefaultSceneRoot`) (`KismetMathLibrary.MakeVector` Distance) false false)))

(fn `Move Up`
  (params (Distance :type "Float (double-precision)" :default 10.0) (ShouldMove :type Boolean :default true))
  (if ShouldMove
    (`SceneComponent.K2_AddRelativeLocation` (`self.DefaultSceneRoot`) (`KismetMathLibrary.MakeVector` 0.0 Distance) false false)))

(fn `UserConstructionScript`)