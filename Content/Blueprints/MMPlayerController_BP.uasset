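; Player controller that drives an MMCamera_BP view target with keyboard panning and mouse-wheel zoom.
; BeginPlay sets game-and-UI input with a locked mouse and caches the camera from the view target.
; The wheel changes the spring arm length by ZoomScale within fixed near and far limits.
; Tick polls WASD every frame and passes key states to the camera's move functions with fixed, frame-rate-independent-unaware distances.
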(event `self.ReceiveBeginPlay`
  (`WidgetBlueprintLibrary.SetInputMode_GameAndUIEx` self null "LockAlways" false)
  (bind _asmmcamera_bp (cast `/Game/Blueprints/MMCamera_BP` (`self.GetViewTarget`)))
  (set `self.MMCamera` _asmmcamera_bp))

(event `Key|MouseScrollUp`
  (params (Key :type "Key Structure"))
  (bind _springarm (`/Game/Blueprints/MMCamera_BP.SpringArm` (`self.MMCamera`)))
  (bind _returnvalue (+ (* (`self.Zoom Scale`) -1.0) (`SpringArmComponent.TargetArmLength` _springarm)))
  (:`Pressed`
    (if (> _returnvalue 200.0)
      (set `SpringArmComponent.TargetArmLength` _returnvalue _springarm))))

(event `Key|MouseScrollDown`
  (params (Key :type "Key Structure"))
  (bind _springarm (`/Game/Blueprints/MMCamera_BP.SpringArm` (`self.MMCamera`)))
  (bind _returnvalue (+ (`SpringArmComponent.TargetArmLength` _springarm) (`self.Zoom Scale`)))
  (:`Pressed`
    (if (< _returnvalue 2500.0)
      (set `SpringArmComponent.TargetArmLength` _returnvalue _springarm))))

(event `self.ReceiveTick`
  (params (DeltaSeconds :type "Float (single-precision)"))
  (bind _mmcamera (`self.MMCamera`))
  (`/Game/Blueprints/MMCamera_BP.Move Left` _mmcamera 10.0 (`self.IsInputKeyDown` "A"))
  (`/Game/Blueprints/MMCamera_BP.Move RIght` _mmcamera -10.0 (`self.IsInputKeyDown` "D"))
  (`/Game/Blueprints/MMCamera_BP.Move Up` _mmcamera 10.0 (`self.IsInputKeyDown` "W"))
  (`/Game/Blueprints/MMCamera_BP.Move Down` _mmcamera -10.0 (`self.IsInputKeyDown` "S")))

(fn `UserConstructionScript`)